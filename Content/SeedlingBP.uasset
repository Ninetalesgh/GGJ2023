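; Seedling minion Blueprint that dresses the seedling in a faction-specific hat, made of front and back sprites.
; When the state component's owning player changes, it prints the new owner's name and reads that player's faction and variation.
; SetupHatMinion then picks sprites by seedling state: planted seedlings get per-variation faction hats, uprooted ones a single faction sprout.
; Only planted Mushroom hats use a back sprite, and unassigned factions clear both.
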(event `self.SeedlingStateComp.OnOwningPlayerChanged`
  (params (Seedling :type "xAICharacter Object Reference") (NewOwningPlayer :type "xCharacter Object Reference") (OldOwningPlayer :type "xCharacter Object Reference"))
  (bind _factioncomp (`xCharacter.FactionComp` NewOwningPlayer))
  (`KismetSystemLibrary.PrintString` (`KismetSystemLibrary.GetDisplayName` NewOwningPlayer))
  (`self.SetupHatMinion` (`self.HatFront`) (`self.HatBackComponent`) (`xFactionComponent.GetFaction` _factioncomp) (`xFactionComponent.GetFactionVariation` _factioncomp) (`xSeedlingStateComponent.State` (`self.SeedlingStateComp`))))

(fn `SetupHatMinion`
  (params (FrontHat :type "PaperSpriteComponent Object Reference") (BackHat :type "PaperSpriteComponent Object Reference") (Faction :type "EFaction Enum" :default "Faction_Unassigned") (Variation :type "EFactionVariation Enum" :default "FactionVariation_0") (SeedlingState :type "ESeedlingState Enum" :default "SeedlingState_Planted"))
  (locals (LocalFrontHat :type "PaperSpriteComponent Object Reference") (LocalBackHat :type "PaperSpriteComponent Object Reference") (Local_Faction :type "EFaction Enum") (LocalVariation :type "EFactionVariation Enum") (LocalSeedlingState :type "ESeedlingState Enum"))
  (set `local.LocalFrontHat` FrontHat)
  (set `local.LocalBackHat` BackHat)
  (set `local.Local_Faction` Faction)
  (set `local.LocalVariation` Variation)
  (set `local.LocalSeedlingState` SeedlingState)
  (switch `ESeedlingState` (`local.LocalSeedlingState`)
    (:`SeedlingState_Planted`
      (switch `EFaction` (`local.Local_Faction`)
        (:`Faction_Unassigned`
          (`PaperSpriteComponent.SetSprite` (`local.LocalFrontHat`) null)
          (`PaperSpriteComponent.SetSprite` (`local.LocalBackHat`) null))
        (:`Faction_Leafy`
          (`PaperSpriteComponent.SetSprite` (`local.LocalFrontHat`) (select `EFactionVariation` (`local.LocalVariation`) :`FactionVariation_0` "/Game/Art/Sprites/leafy_faction/hat_minion_leafy1_Sprite.hat_minion_leafy1_Sprite" :`FactionVariation_1` "/Game/Art/Sprites/leafy_faction/hat_minion_leafy2_Sprite.hat_minion_leafy2_Sprite" :!type "PaperSprite Object Reference"))
          (`PaperSpriteComponent.SetSprite` (`local.LocalBackHat`) (select `EFactionVariation` (`local.LocalVariation`) :!type "PaperSprite Object Reference")))
        (:`Faction_Succulent`
          (`PaperSpriteComponent.SetSprite` (`local.LocalFrontHat`) (select `EFactionVariation` (`local.LocalVariation`) :`FactionVariation_0` "/Game/Art/Sprites/succulent_faction/hat_minion_succulent1_Sprite.hat_minion_succulent1_Sprite" :`FactionVariation_1` "/Game/Art/Sprites/succulent_faction/hat_minion_succulent2_Sprite.hat_minion_succulent2_Sprite" :!type "PaperSprite Object Reference"))
          (`PaperSpriteComponent.SetSprite` (`local.LocalBackHat`) null))
        (:`Faction_Mushroom`
          (`PaperSpriteComponent.SetSprite` (`local.LocalFrontHat`) (select `EFactionVariation` (`local.LocalVariation`) :`FactionVariation_0` "/Game/Art/Sprites/mushroom_faction/hat_minion_mushroom1_front_Sprite.hat_minion_mushroom1_front_Sprite" :`FactionVariation_1` "/Game/Art/Sprites/mushroom_faction/hat_minion_mushroom2_front_Sprite.hat_minion_mushroom2_front_Sprite" :!type "PaperSprite Object Reference"))
          (`PaperSpriteComponent.SetSprite` (`local.LocalBackHat`) (select `EFactionVariation` (`local.LocalVariation`) :`FactionVariation_0` "/Game/Art/Sprites/mushroom_faction/hat_minion_mushroom1_back_Sprite.hat_minion_mushroom1_back_Sprite" :`FactionVariation_1` "/Game/Art/Sprites/mushroom_faction/hat_minion_mushroom2_back_Sprite.hat_minion_mushroom2_back_Sprite" :!type "PaperSprite Object Reference")))
        (:`Faction_Flower`
          (`PaperSpriteComponent.SetSprite` (`local.LocalFrontHat`) (select `EFactionVariation` (`local.LocalVariation`) :`FactionVariation_0` "/Game/Art/Sprites/flower_faction/hat_minion_flower1_Sprite.hat_minion_flower1_Sprite" :`FactionVariation_1` "/Game/Art/Sprites/flower_faction/hat_minion_flower2_Sprite.hat_minion_flower2_Sprite" :!type "PaperSprite Object Reference"))
          (`PaperSpriteComponent.SetSprite` (`local.LocalBackHat`) null))))
    (:`SeedlingState_Uprooted`
      (switch `EFaction` (`local.Local_Faction`)
        (:`Faction_Unassigned`
          (`PaperSpriteComponent.SetSprite` (`local.LocalFrontHat`) null)
          (`PaperSpriteComponent.SetSprite` (`local.LocalBackHat`) null))
        (:`Faction_Leafy`
          (`PaperSpriteComponent.SetSprite` (`local.LocalFrontHat`) "/Game/Art/Sprites/leafy_faction/hat_minion_leaf_sprout_Sprite.hat_minion_leaf_sprout_Sprite")
          (`PaperSpriteComponent.SetSprite` (`local.LocalBackHat`) null))
        (:`Faction_Succulent`
          (`PaperSpriteComponent.SetSprite` (`local.LocalFrontHat`) "/Game/Art/Sprites/succulent_faction/hat_minion_succulent_sprout_Sprite.hat_minion_succulent_sprout_Sprite")
          (`PaperSpriteComponent.SetSprite` (`local.LocalBackHat`) null))
        (:`Faction_Mushroom`
          (`PaperSpriteComponent.SetSprite` (`local.LocalFrontHat`) "/Game/Art/Sprites/mushroom_faction/hat_minion_mushroom_sprout_Sprite.hat_minion_mushroom_sprout_Sprite")
          (`PaperSpriteComponent.SetSprite` (`local.LocalBackHat`) null))
        (:`Faction_Flower`
          (`PaperSpriteComponent.SetSprite` (`local.LocalFrontHat`) "/Game/Art/Sprites/flower_faction/hat_minion_flower_sprout_Sprite.hat_minion_flower_sprout_Sprite")
          (`PaperSpriteComponent.SetSprite` (`local.LocalBackHat`) null))))))

(fn `UserConstructionScript`)