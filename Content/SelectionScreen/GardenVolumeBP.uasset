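; Selection-screen garden room volume that assigns a faction to the player who enters it.
; On enter overlap, if no faction is given yet, it shows the door, enables its hex collision, then checks for the player.
; The EFaction value picks the hat buff action added through ActionComp and the matching coloured transformation Niagara burst.
; Exit overlap is empty, leaving the door-open and unassign logic unconnected.
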(event `self.ReceiveBeginPlay`
  (bind _vfx_colours (`self.VFX_Colours`))
  ;[1 1 1] On Load
  (`SceneComponent.SetVisibility` (`self.DoorUp`) false false)
  (`PrimitiveComponent.SetCollisionEnabled` (`self.HexCollision`) "NoCollision")
  (`KismetArrayLibrary.Array_Add` _vfx_colours "/Game/Niagara/Done/Green/NS_TransformationGreen.NS_TransformationGreen")
  (`KismetArrayLibrary.Array_Add` _vfx_colours "/Game/Niagara/Done/Purple/NS_TransformationPurple.NS_TransformationPurple")
  (`KismetArrayLibrary.Array_Add` _vfx_colours "/Game/Niagara/Done/Red/NS_TransformationRed.NS_TransformationRed")
  (`KismetArrayLibrary.Array_Add` _vfx_colours "/Game/Niagara/Done/Yellow/NS_TransformationYellow.NS_TransformationYellow"))

(event `self.PlayerExit.OnComponentBeginOverlap`
  (params (OverlappedComponent :type "PrimitiveComponent Object Reference") (OtherActor :type "Actor Object Reference") (OtherComp :type "PrimitiveComponent Object Reference") (OtherBodyIndex :type Integer) (bFromSweep :type Boolean) (SweepResult :type "HitResult Structure (by ref)"))
  ;[1 1 1] Player has exited
)

(event `self.PlayerEnter.OnComponentBeginOverlap`
  (params (OverlappedComponent :type "PrimitiveComponent Object Reference") (OtherActor :type "Actor Object Reference") (OtherComp :type "PrimitiveComponent Object Reference") (OtherBodyIndex :type Integer) (bFromSweep :type Boolean) (SweepResult :type "HitResult Structure (by ref)"))
  (bind _playercharacter (`self.PlayerCharacter`))
  (bind _actioncomp (`xCharacter.ActionComp` _playercharacter))
  ;[1 1 1] Player enters room
  ;[1 1 1] Bool Check
  (if (not (`self.GivenFaction`))
    (`self.CloseDoor`
      (:`Done`
        ;[1 1 1] Check If Player
        (if (== (`GameplayStatics.GetObjectClass` OtherActor) "/Game/PlayerCharacterBP.PlayerCharacterBP_C")
          (bind _asplayer_character_bp (cast `/Game/PlayerCharacterBP` OtherActor))
          (set `self.PlayerCharacter` _asplayer_character_bp)
          ;[1 1 1] Set Faction
          (switch `EFaction` (`self.EFaction`)
            (:`Faction_Leafy`
              (`xActionComponent.AddAction` _actioncomp _playercharacter "/Game/Actions/Buff_Hat1LeafBP.Buff_Hat1LeafBP_C")
              (set `self.ColourInt` 0))
            (:`Faction_Succulent`
              (`xActionComponent.AddAction` _actioncomp _playercharacter "/Game/Actions/Buff_Hat2SucculentBP.Buff_Hat2SucculentBP_C")
              (set `self.ColourInt` 1))
            (:`Faction_Mushroom`
              (`xActionComponent.AddAction` _actioncomp _playercharacter "/Game/Actions/Buff_Hat3MushroomBP.Buff_Hat3MushroomBP_C")
              (set `self.ColourInt` 2))
            (:`Faction_Flower`
              (`xActionComponent.AddAction` _actioncomp _playercharacter "/Game/Actions/Buff_Hat4FlowerBP.Buff_Hat4FlowerBP_C")
              (set `self.ColourInt` 3)))
          (set `self.GivenFaction` true)
          (`self.EffectFromArray` (`|GetArrayItem` (`self.VFX_Colours`) (`self.ColourInt`)) (`SceneComponent.K2_GetComponentLocation` (`Character.Mesh` (`self.PlayerCharacter`))))
          (`GameplayStatics.PlaySound2D` "/Game/Levels/Sounds/sounds/13_Hair_change_-_Bubble_SE4.13_Hair_change_-_Bubble_SE4" 1.0 (`KismetMathLibrary.RandomFloatInRange` 0.8 1.2) 0.0 null null)
          (else
            (`KismetSystemLibrary.PrintString` "Not a player" true true (struct :`R` 1.0 :`B` 0.393823 :`A` 1.0))))))))

(fn `Countdown w/ Text`
  (params (`No. of Seconds` :type Integer) (Text :type "Object Object Reference"))
  (locals (NewLocalVar :type Integer))
  (for _index (range 1 (+ `No. of Seconds` 1))
    ;[1 1 1] Play Sound, Update Text, wait 1 sec
    (`GameplayStatics.PlaySound2D` "/Engine/VREditor/Sounds/UI/Flashlight_Switch.Flashlight_Switch" 1.0 1.0 0.0 null null))
  ;[1 1 1] When countdown done, print final text, wait, empty.
  (`GameplayStatics.PlaySound2D` "/Engine/VREditor/Sounds/UI/Object_PickUp.Object_PickUp" 1.0 1.0 0.0 null null))

(fn `UserConstructionScript`)