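; Selection-screen actor that runs the four-player ready check and the camera move that follows it.
; Each player's trigger overlap passes through a PlayerCharacterBP class check to set a ready flag, and end overlap restores PhysicsOnly collision on that player's door cube.
; Tick polls the flags; once all are ready, it hides the hexes, disables door collision, and plays a timeline that lerps the CineCamera toward CameraEndLocation, then clears the text.
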(event `self.ReceiveBeginPlay`)

(event `self.ReceiveTick`
  (params (DeltaSeconds :type "Float (single-precision)"))
  (`self.Check if all ready`)
  (`SceneComponent.SetVisibility` (`self.hex_03`) false false)
  (`SceneComponent.SetVisibility` (`self.hex_02`) false false)
  (`SceneComponent.SetVisibility` (`self.hex_01`) false false)
  (`SceneComponent.SetVisibility` (`self.hex_04`) false false)
  ;[1 1 1] Pan Camera
  (`self.SetAllCollisions`)
  (bind (_direction _pan) (`Timeline|CameraPan` :!via `PlayFromStart`)
    (:`Update`
      (`SceneComponent.K2_SetWorldLocation` (`self.CineCamera`) (`KismetMathLibrary.VLerp` (`SceneComponent.K2_GetComponentLocation` (`self.CineCamera`)) (`SceneComponent.K2_GetComponentLocation` (`self.CameraEndLocation`)) _pan) false false))
    (:`Finished`
      (`TextRenderComponent.K2_SetText` (`self.TextRead`) ""))))

(event `self.Player 1.OnComponentBeginOverlap`
  (params (OverlappedComponent :type "PrimitiveComponent Object Reference") (OtherActor :type "Actor Object Reference") (OtherComp :type "PrimitiveComponent Object Reference") (OtherBodyIndex :type Integer) (bFromSweep :type Boolean) (SweepResult :type "HitResult Structure (by ref)"))
  ;[1 1 1] ReadyCehck
  (`self.Check player` (`self.PlayerReady_1`) OtherActor)
  (set `self.PlayerReady_1` true))

(event `self.Player 1.OnComponentEndOverlap`
  (params (OverlappedComponent :type "PrimitiveComponent Object Reference") (OtherActor :type "Actor Object Reference") (OtherComp :type "PrimitiveComponent Object Reference") (OtherBodyIndex :type Integer))
  ;[1 1 1] Close doors
  (`PrimitiveComponent.SetCollisionEnabled` (`self.Cube`) "PhysicsOnly"))

(event `self.Player 2.OnComponentBeginOverlap`
  (params (OverlappedComponent :type "PrimitiveComponent Object Reference") (OtherActor :type "Actor Object Reference") (OtherComp :type "PrimitiveComponent Object Reference") (OtherBodyIndex :type Integer) (bFromSweep :type Boolean) (SweepResult :type "HitResult Structure (by ref)"))
  ;[1 1 1] ReadyCehck
  (`self.Check player` (`self.PlayerReady_2`) OtherActor)
  (set `self.PlayerReady_2` true))

(event `self.Player 2.OnComponentEndOverlap`
  (params (OverlappedComponent :type "PrimitiveComponent Object Reference") (OtherActor :type "Actor Object Reference") (OtherComp :type "PrimitiveComponent Object Reference") (OtherBodyIndex :type Integer))
  ;[1 1 1] Close doors
  (`PrimitiveComponent.SetCollisionEnabled` (`self.Cube1`) "PhysicsOnly"))

(event `self.Player 3.OnComponentEndOverlap`
  (params (OverlappedComponent :type "PrimitiveComponent Object Reference") (OtherActor :type "Actor Object Reference") (OtherComp :type "PrimitiveComponent Object Reference") (OtherBodyIndex :type Integer))
  ;[1 1 1] Close doors
  (`PrimitiveComponent.SetCollisionEnabled` (`self.Cube2`) "PhysicsOnly"))

(event `self.Player 3.OnComponentBeginOverlap`
  (params (OverlappedComponent :type "PrimitiveComponent Object Reference") (OtherActor :type "Actor Object Reference") (OtherComp :type "PrimitiveComponent Object Reference") (OtherBodyIndex :type Integer) (bFromSweep :type Boolean) (SweepResult :type "HitResult Structure (by ref)"))
  ;[1 1 1] ReadyCehck
  (`self.Check player` (`self.PlayerReady_3`) OtherActor)
  (set `self.PlayerReady_3` true))

(event `self.Player 4.OnComponentEndOverlap`
  (params (OverlappedComponent :type "PrimitiveComponent Object Reference") (OtherActor :type "Actor Object Reference") (OtherComp :type "PrimitiveComponent Object Reference") (OtherBodyIndex :type Integer))
  ;[1 1 1] Close doors
  (`PrimitiveComponent.SetCollisionEnabled` (`self.Cube3`) "PhysicsOnly"))

(event `self.Player 4.OnComponentBeginOverlap`
  (params (OverlappedComponent :type "PrimitiveComponent Object Reference") (OtherActor :type "Actor Object Reference") (OtherComp :type "PrimitiveComponent Object Reference") (OtherBodyIndex :type Integer) (bFromSweep :type Boolean) (SweepResult :type "HitResult Structure (by ref)"))
  ;[1 1 1] ReadyCehck
  (`self.Check player` (`self.PlayerReady_4`) OtherActor)
  (set `self.PlayerReady_4` true))

(fn `UserConstructionScript`)