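; Player character Blueprint that dresses the character in a two-layer sprite hat matching its faction and variation.
; The construction script snaps the hat base to a socket on the body component.
; The faction component's change event drives SetupHat, which selects front and back sprites per faction, clearing those without art.
; An unconnected authority switch for setting or reading the initial faction never runs.
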(event `self.ReceiveBeginPlay`
  (add `xFactionComponent.OnFactionChanged` (`self.FactionComp`) (delegate `FactionChanged`)))

(event `FactionChanged`
  (params (Instigator :type "Actor Object Reference") (NewFaction :type "EFaction Enum" :default "Faction_Unassigned") (NewVariation :type "EFactionVariation Enum" :default "FactionVariation_0") (OldFaction :type "EFaction Enum" :default "Faction_Unassigned") (OldVariation :type "EFactionVariation Enum" :default "FactionVariation_0"))
  (`self.SetupHat` (`self.HatFront`) (`self.HatBackComponent`) NewFaction NewVariation))

(fn `SetupHat`
  (params (FrontHat :type "PaperSpriteComponent Object Reference") (BackHat :type "PaperSpriteComponent Object Reference") (Faction :type "EFaction Enum" :default "Faction_Unassigned") (Variation :type "EFactionVariation Enum" :default "FactionVariation_0"))
  (locals (Local_Faction :type "EFaction Enum" :default "Faction_Unassigned") (LocalFrontHat :type "PaperSpriteComponent Object Reference") (LocalBackHat :type "PaperSpriteComponent Object Reference") (LocalVariation :type "EFactionVariation Enum" :default "FactionVariation_0"))
  (set `local.LocalFrontHat` FrontHat)
  (set `local.LocalBackHat` BackHat)
  (set `local.Local_Faction` Faction)
  (set `local.LocalVariation` Variation)
  (switch `EFaction` (`local.Local_Faction`)
    (:`Faction_Unassigned`
      (`PaperSpriteComponent.SetSprite` (`local.LocalFrontHat`) null)
      (`PaperSpriteComponent.SetSprite` (`local.LocalBackHat`) null))
    (:`Faction_Leafy`
      (`PaperSpriteComponent.SetSprite` (`local.LocalFrontHat`) (select `EFactionVariation` (`local.LocalVariation`) :`FactionVariation_0` "/Game/Art/Sprites/leafy_faction/hat_leafy1_front_Sprite.hat_leafy1_front_Sprite" :`FactionVariation_1` "/Game/Art/Sprites/leafy_faction/hat_leafy2_Sprite.hat_leafy2_Sprite" :!type "PaperSprite Object Reference"))
      (`PaperSpriteComponent.SetSprite` (`local.LocalBackHat`) (select `EFactionVariation` (`local.LocalVariation`) :`FactionVariation_0` "/Game/Art/Sprites/leafy_faction/hat_leafy1_back_Sprite.hat_leafy1_back_Sprite" :!type "PaperSprite Object Reference")))
    (:`Faction_Succulent`
      (`PaperSpriteComponent.SetSprite` (`local.LocalFrontHat`) (select `EFactionVariation` (`local.LocalVariation`) :`FactionVariation_0` "/Game/Art/Sprites/succulent_faction/hat_succulent1_Sprite.hat_succulent1_Sprite" :`FactionVariation_1` "/Game/Art/Sprites/succulent_faction/hat_succulent2_Sprite.hat_succulent2_Sprite" :!type "PaperSprite Object Reference"))
      (`PaperSpriteComponent.SetSprite` (`local.LocalBackHat`) null))
    (:`Faction_Mushroom`
      (`PaperSpriteComponent.SetSprite` (`local.LocalFrontHat`) (select `EFactionVariation` (`local.LocalVariation`) :`FactionVariation_0` "/Game/Art/Sprites/mushroom_faction/hat_mushroom1_front_Sprite.hat_mushroom1_front_Sprite" :`FactionVariation_1` "/Game/Art/Sprites/mushroom_faction/hat_mushroom2_front_Sprite.hat_mushroom2_front_Sprite" :!type "PaperSprite Object Reference"))
      (`PaperSpriteComponent.SetSprite` (`local.LocalBackHat`) (select `EFactionVariation` (`local.LocalVariation`) :`FactionVariation_0` "/Game/Art/Sprites/mushroom_faction/hat_mushroom1_back_Sprite.hat_mushroom1_back_Sprite" :`FactionVariation_1` "/Game/Art/Sprites/mushroom_faction/hat_mushroom2_back_Sprite.hat_mushroom2_back_Sprite" :!type "PaperSprite Object Reference")))
    (:`Faction_Flower`
      (`PaperSpriteComponent.SetSprite` (`local.LocalFrontHat`) (select `EFactionVariation` (`local.LocalVariation`) :`FactionVariation_0` "/Game/Art/Sprites/flower_faction/hat_flower1_Sprite.hat_flower1_Sprite" :`FactionVariation_1` "/Game/Art/Sprites/flower_faction/hat_flower2_Sprite.hat_flower2_Sprite" :!type "PaperSprite Object Reference"))
      (`PaperSpriteComponent.SetSprite` (`local.LocalBackHat`) null))))

(fn `UserConstructionScript`
  (`SceneComponent.K2_AttachToComponent` (`self.HatBase`) (`self.BodyComp`) (`self.Hat_Socket`) "SnapToTarget" "SnapToTarget" "KeepWorld" false))