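; A hex grid tile Blueprint that changes its look to match the faction that holds it.
; When its faction component reports a change, a switch on the new faction sets the tile's static mesh and first material slot.
; Unassigned tiles show a concrete hex, while the Leafy, Succulent, Mushroom and Flower factions share a neutral low mesh with their own biome material.
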(event `self.FactionComp.OnFactionChanged`
  (params (Instigator :type "Actor Object Reference") (NewFaction :type "EFaction Enum" :default "Faction_Unassigned") (NewVariation :type "EFactionVariation Enum" :default "FactionVariation_0") (OldFaction :type "EFaction Enum" :default "Faction_Unassigned") (OldVariation :type "EFactionVariation Enum" :default "FactionVariation_0"))
  (switch `EFaction` NewFaction
    (:`Faction_Unassigned`
      (`StaticMeshComponent.SetStaticMesh` (`self.MeshComp`) "/Game/Art/Assets/hex_01.hex_01")
      (`PrimitiveComponent.SetMaterial` (`self.MeshComp`) 0 "/Game/Art/Materials/MI_Concrete.MI_Concrete"))
    (:`Faction_Leafy`
      (`StaticMeshComponent.SetStaticMesh` (`self.MeshComp`) "/Game/Art/Assets/Hexes/neutral_low.neutral_low")
      (`PrimitiveComponent.SetMaterial` (`self.MeshComp`) 0 "/Game/Art/Assets/Hexes/MI_Leaves_Biome_Hex.MI_Leaves_Biome_Hex"))
    (:`Faction_Succulent`
      (`StaticMeshComponent.SetStaticMesh` (`self.MeshComp`) "/Game/Art/Assets/Hexes/neutral_low.neutral_low")
      (`PrimitiveComponent.SetMaterial` (`self.MeshComp`) 0 "/Game/Art/Assets/SuculentBiome/MI_Succulent_Hexes.MI_Succulent_Hexes"))
    (:`Faction_Mushroom`
      (`StaticMeshComponent.SetStaticMesh` (`self.MeshComp`) "/Game/Art/Assets/Hexes/neutral_low.neutral_low")
      (`PrimitiveComponent.SetMaterial` (`self.MeshComp`) 0 "/Game/Art/Assets/Hexes/MI_Shroom_Hexes.MI_Shroom_Hexes"))
    (:`Faction_Flower`
      (`StaticMeshComponent.SetStaticMesh` (`self.MeshComp`) "/Game/Art/Assets/Hexes/neutral_low.neutral_low")
      (`PrimitiveComponent.SetMaterial` (`self.MeshComp`) 0 "/Game/Art/Assets/FlowerBiome/MI_Flowers_Biome.MI_Flowers_Biome"))))

(fn `UserConstructionScript`)